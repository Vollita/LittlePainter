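; Interactable box actor that is destroyed when the F button event fires while something overlaps it.
; Begin overlap sets a collision flag, shows the interaction widget held by BP_PlayerController_Child and binds the box's handler to that controller's F-button event.
; End overlap clears the flag and removes the widget but leaves the binding, so the flag gates destruction.
; Neither overlap event checks which actor triggered it.
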(event Custom|F_Button_Event
  (if (Variables|Default|GetIsCollision)
    (Actor|DestroyActor)))

(event EventBeginPlay)

(event Collision|EventActorBeginOverlap
  (params (OtherActor :type Actor%20Object%20Reference))
  (Variables|Default|SetIsCollision true)
  (bind _asbp_player_controller_child (Utilities|Casting|CastToBP_PlayerController_Child (Game|GetPlayerController 0)))
  (UserInterface|Viewport|AddtoViewport (Variables|/Game/ThirdPerson/Blueprints/BP_PlayerController_Child.BP_PlayerController_Child_C|GetUIBP_interacton _asbp_player_controller_child) 0)
  (EventDispatchers|BindEventtoFButton _asbp_player_controller_child (delegate Custom|F_Button_Event)))

(event EventTick
  (params (DeltaSeconds :type Float%20%28single-precision%29)))

(event Collision|EventActorEndOverlap
  (params (OtherActor :type Actor%20Object%20Reference))
  (Variables|Default|SetIsCollision false)
  (bind _asbp_player_controller_child (Utilities|Casting|CastToBP_PlayerController_Child (Game|GetPlayerController 0)))
  (Widget|RemovefromParent (Variables|/Game/ThirdPerson/Blueprints/BP_PlayerController_Child.BP_PlayerController_Child_C|GetUIBP_interacton _asbp_player_controller_child)))

(fn ConstructionScript)